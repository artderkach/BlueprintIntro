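; Interactive lamp Blueprint that lets the player switch a spotlight with the F key while near it.
; Overlapping LampTrigger enables input for player controller 0 and leaving disables it, with both events toggling the help text's visibility.
; Pressing F toggles the spotlight's visibility and stops or starts the lamp sound based on whether it is playing.
; The trigger events do not check which actor overlaps.
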(event OnComponentBeginOverlap(LampTrigger)
  (params (OverlappedComponent :type Primitive%20Component%20Object%20Reference) (OtherActor :type Actor%20Object%20Reference) (OtherComp :type Primitive%20Component%20Object%20Reference) (OtherBodyIndex :type Integer) (bFromSweep :type Boolean) (SweepResult :type Hit%20Result%20Structure%20%28by%20ref%29))
  ;[0.6457 0.8565 1] Trigger overlap - enable/disable input
  (Input|EnableInput (Game|GetPlayerController 0))
  (Rendering|ToggleVisibility (Variables|Default|GetLampHelpText) false))

(event OnComponentEndOverlap(LampTrigger)
  (params (OverlappedComponent :type Primitive%20Component%20Object%20Reference) (OtherActor :type Actor%20Object%20Reference) (OtherComp :type Primitive%20Component%20Object%20Reference) (OtherBodyIndex :type Integer))
  ;[0.6457 0.8565 1] Trigger overlap - enable/disable input
  (Input|DisableInput (Game|GetPlayerController 0))
  (Rendering|ToggleVisibility (Variables|Default|GetLampHelpText) false))

(event EventBeginPlay)

(event Collision|EventActorBeginOverlap
  (params (OtherActor :type Actor%20Object%20Reference)))

(event EventTick
  (params (DeltaSeconds :type Float%20%28single-precision%29)))

(event Input|KeyboardEvents|F
  (params (Key :type Key%20Structure :default "AnyKey"))
  (bind _lampsound (Variables|Default|GetLampSound))
  ;[1 0.8503 0.627] Press 'F' to toggle light
  (:Pressed
    (Rendering|ToggleVisibility (Variables|Default|GetLampSpotLight) false)
    (if (Audio|Components|Audio|IsPlaying (Variables|Default|GetLampSound))
      (Audio|Components|Audio|Stop _lampsound)
      (else
        (Audio|Components|Audio|Play _lampsound 0.0)))))

(fn ConstructionScript)